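; Grind railing actor that starts a straight, non-curved grind when the third-person character lands on it.
; On BeginPlay it gathers every Billboard component under its root as a checkpoint list and prints the count for debugging.
; When a falling character overlaps ColliderA, it passes the checkpoints and the mesh's world location to the character's CEGrinding event, leaving the grind itself to the character.
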(event OnComponentBeginOverlap(ColliderA)
  (params (OverlappedComponent :type Primitive%20Component%20Object%20Reference) (OtherActor :type Actor%20Object%20Reference) (OtherComp :type Primitive%20Component%20Object%20Reference) (OtherBodyIndex :type Integer) (bFromSweep :type Boolean) (SweepResult :type Hit%20Result%20Structure%20%28by%20ref%29))
  (bind _asbp_third_person_character (Utilities|Casting|CastToBP_ThirdPersonCharacter OtherActor))
  (if (AI|Components|NavMovement|IsFalling (Variables|/Script/Engine.Character|GetCharacterMovement _asbp_third_person_character))
    (Default|CEGrinding _asbp_third_person_character false (Transformation|GetWorldLocation (Variables|Default|GetStaticMesh)) (Variables|Default|GetCheckpoints))))

(event EventBeginPlay
  (bind _checkpoints (Variables|Default|GetCheckpoints))
  (for _array_element (Components|GetChildrenComponents (Variables|Default|GetDefaultSceneRoot) true)
    (bind _asbillboard_component (Utilities|Casting|CastToBillboardComponent _array_element))
    (Utilities|Array|Add _checkpoints _asbillboard_component))
  (Development|PrintString (Utilities|String|ToString(Integer) (Utilities|Array|Length _checkpoints))))

(event Collision|EventActorBeginOverlap
  (params (OtherActor :type Actor%20Object%20Reference)))

(event EventTick
  (params (DeltaSeconds :type Float%20%28single-precision%29)))

(fn ConstructionScript)