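; Grindable rail actor that a player can grind along, shaped by an editable spline.
; The construction script adds a spline mesh segment between each pair of spline points, keeping only the last one in the SplineMesh variable.
; GetSplineDirection returns the spline, that mesh, stored direction and offset, plus a start distance found by brute-force sampling for the point nearest the hit.
; CanGrind always returns true, and the event graph is empty.
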(event EventBeginPlay)

(event Collision|EventActorBeginOverlap
  (params (OtherActor :type Actor%20Object%20Reference)))

(event EventTick
  (params (DeltaSeconds :type Float%20%28single-precision%29)))

(fn ConstructionScript
  (bind _spline (Variables|Default|GetSpline))
  (for _index (range 0 (- (Spline|GetNumberOfSplinePoints _spline) 2))
    (bind _returnvalue (AddComponent|AddSplineMeshComponent false))
    (bind _output_get (Variables|Default|SetSplineMesh _returnvalue))
    (SplineMesh|SetStartandEnd _output_get (.Location (Spline|GetLocationandTangentatSplinePoint _spline _index "Local")) (.Tangent (Spline|GetLocationandTangentatSplinePoint _spline _index "Local")) (.Location (Spline|GetLocationandTangentatSplinePoint _spline (+ _index 1) "Local")) (.Tangent (Spline|GetLocationandTangentatSplinePoint _spline (+ _index 1) "Local")) true :!class /Script/Engine.SplineMeshComponent)))

(fn GetObjectDistanceAlongSpline
  (params (Location :type Vector))
  (if (< (Math|Vector|Distance(Vector) Location (Spline|GetLocationatDistanceAlongSpline (Variables|Default|GetSpline) (LocalVariables|GetLocalDistance) "World")) (LocalVariables|GetLocalMinDistance)) :!label _label
    (LocalVariables|SetLocalMinDistance (Math|Vector|Distance(Vector) Location (Spline|GetLocationatDistanceAlongSpline (Variables|Default|GetSpline) (LocalVariables|GetLocalDistance) "World")))
    (LocalVariables|SetLocalClosestDistance (LocalVariables|GetLocalDistance)))
  (LocalVariables|SetLocalDistance (+ (LocalVariables|GetLocalDistance) 1e+01))
  (if (< (LocalVariables|GetLocalDistance) (Spline|GetSplineLength (Variables|Default|GetSpline)))
    (goto _label)
    (else
      (return (LocalVariables|GetLocalClosestDistance)))))

(fn CanGrind?
  (return true))

(fn GetSplineDirection
  (params (HitLocation :type Vector :default "0, 0, 0"))
  (bind _spline_distance (CallFunction|GetObjectDistanceAlongSpline HitLocation))
  (return (Variables|Default|GetSpline) (Variables|Default|GetSplineMesh) _spline_distance (Variables|Default|GetDirection) (Variables|Default|GetGrind%20Offset)))